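; Holdable baseball bat that hits BP_Ball_Baseball actors it overlaps.
; While held, a 60 Hz looping timer sweeps a physics-simulated hit Box to the bat mesh's transform to catch contacts missed between frames.
; On overlap, the ball's velocity is replaced by the Box's scaled velocity and a metal bat sound plays with speed-based volume.
; Releasing the bat pauses the timer, stops Box simulation and resets its relative transform.
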(event `self.ReceiveBeginPlay`
  ;[0 1 0] Begin Play
  (`parent.ReceiveBeginPlay`)
  (bind _returnvalue (`KismetSystemLibrary.K2_SetTimerDelegate` (delegate `CheckBetweenFrames`) 0.016667 true))
  (bind _output_get (set `self.EventTimer` _returnvalue))
  (`KismetSystemLibrary.K2_PauseTimerHandle` _output_get))

(event `self.SpecialHeldConditions`
  (params (IsHeld :type Boolean))
  (bind _eventtimer (`self.EventTimer`))
  (bind _box (`self.Box`))
  ;[1 1 1] Override special conditions
  (if IsHeld
    (`KismetSystemLibrary.K2_UnPauseTimerHandle` _eventtimer)
    (`PrimitiveComponent.SetSimulatePhysics` _box true)
    (else
      (`KismetSystemLibrary.K2_PauseTimerHandle` _eventtimer)
      (`PrimitiveComponent.SetSimulatePhysics` _box false)
      (`SceneComponent.K2_SetRelativeLocationAndRotation` :`self` (`self.Box`) :`NewLocation` (0.0 0.0 9.0)))))

(event `CheckBetweenFrames`
  (bind _staticmeshcomponent (`self.StaticMeshComponent`))
  ;[1 1 1] Do a sweep check tro catch missed things between frames
  (`SceneComponent.K2_SetWorldLocationAndRotation` (`self.Box`) (+ (`SceneComponent.K2_GetComponentLocation` _staticmeshcomponent) (* (`SceneComponent.GetUpVector` _staticmeshcomponent) 9.0)) (`SceneComponent.K2_GetComponentRotation` _staticmeshcomponent) true false))

(event `self.Box.OnComponentBeginOverlap`
  (params (OverlappedComponent :type "PrimitiveComponent Object Reference") (OtherActor :type "Actor Object Reference") (OtherComp :type "PrimitiveComponent Object Reference") (OtherBodyIndex :type Integer) (bFromSweep :type Boolean) (SweepResult :type "HitResult Structure (by ref)"))
  (bind _returnvalue (`SceneComponent.GetComponentVelocity` (`self.Box`)))
  ;[1 1 1] Hit baseballs
  (bind _asbp_ball_baseball (cast `/Game/Blueprints/BP_Ball_Baseball` OtherActor))
  (`PrimitiveComponent.SetPhysicsLinearVelocity` (`StaticMeshActor.StaticMeshComponent` _asbp_ball_baseball) (* _returnvalue 3000.0) false "None")
  (`GameplayStatics.PlaySoundAtLocation` "/Game/SFX/SCue_Bat_Metal.SCue_Bat_Metal" (`self.K2_GetActorLocation`) (struct) (`KismetMathLibrary.MapRangeClamped` (`KismetMathLibrary.VSize` _returnvalue) 0.0 20.0 0.8 1.0) 1.0 0.0 "/Game/SFX/SoundAttenuation.SoundAttenuation" null null))

(fn `UserConstructionScript`
  (`parent.UserConstructionScript`))