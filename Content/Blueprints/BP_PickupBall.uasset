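; BP_PickupBall is a physics ball that BP_MotionController can pick up and drop.
; Pickup disables physics and attaches the ball to the given component, while Drop restores physics and detaches it, both keeping world transform.
; Hits above an impulse threshold print the impulse and play audio with volume scaled to impact strength, throttled by a DoOnce and short Delay.
; The construction script applies the BallMesh.
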(event `/Game/Blueprints/PickupActorInterface.Pickup`
  (params (AttachTo :type "SceneComponent Object Reference"))
  (`PrimitiveComponent.SetSimulatePhysics` (`self.StaticMeshComponent`) false)
  (`SceneComponent.K2_AttachToComponent` (`self.K2_GetRootComponent`) AttachTo "None" "KeepWorld" "KeepWorld" "KeepWorld" false))

(event `/Game/Blueprints/PickupActorInterface.Drop`
  (`PrimitiveComponent.SetSimulatePhysics` (`self.StaticMeshComponent`) true)
  (`self.K2_DetachFromActor` "KeepWorld" "KeepWorld" "KeepWorld"))

(event `self.ReceiveHit`
  (params (MyComp :type "PrimitiveComponent Object Reference") (Other :type "Actor Object Reference") (OtherComp :type "PrimitiveComponent Object Reference") (bSelfMoved :type Boolean) (HitLocation :type "Vector Structure") (HitNormal :type "Vector Structure") (NormalImpulse :type "Vector Structure") (Hit :type "HitResult Structure (by ref)"))
  (bind _returnvalue (`KismetMathLibrary.VSize` NormalImpulse))
  (bind _audio (`self.Audio`))
  (`/Engine/EditorBlueprintResources/StandardMacros.DoOnce` false :!label _label
    (:`Completed`
      (if (> _returnvalue 50.0)
        (`KismetSystemLibrary.PrintString` (`KismetStringLibrary.Conv_DoubleToString` _returnvalue))
        (`AudioComponent.SetVolumeMultiplier` _audio (`KismetMathLibrary.MapRangeClamped` _returnvalue 50.0 5000.0 0.05 1.0))
        (`AudioComponent.Play` _audio 0.0))
      (`KismetSystemLibrary.Delay` 0.2)
      (goto _label :!via `Reset`))))

(fn `UserConstructionScript`
  (`StaticMeshComponent.SetStaticMesh` (`self.StaticMeshComponent`) (`self.BallMesh`)))