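; BP_Tire_Slide is a tire actor that slides along an InterpToMovement path.
; Its construction script runs the parent's, then adds a relative control point on local +Y or -X, chosen by MoveDirection.
; BeginPlay starts a looping timer with a slightly randomized interval of about one second, bound to an UpdateScore event that is empty here.
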(event `self.ReceiveBeginPlay`
  (`KismetSystemLibrary.K2_SetTimerDelegate` (delegate `Update Score`) (`KismetMathLibrary.RandomFloatInRange` 1.0 1.1) true))

(event `Update Score`)

(fn `UserConstructionScript`
  (bind _controlpoints (`InterpToMovementComponent.ControlPoints` (`self.InterpToMovement`)))
  (`parent.UserConstructionScript`)
  (if (`self.MoveDirection`)
    (`KismetArrayLibrary.Array_Add` _controlpoints (make `InterpControlPoint` (0.0 300.0 0.0)))
    (else
      (`KismetArrayLibrary.Array_Add` _controlpoints (make `InterpControlPoint` (-300.0 0.0 0.0))))))