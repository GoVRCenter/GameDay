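; Game mode for GameDay that tracks a score and mirrors it on up to two in-world scoreboards.
; On BeginPlay it finds the BP_Scoreboard actors and caches the Scoreboard widgets from the first two.
; AddToScore updates Score and writes it to each valid widget.
; ResetScore writes Score to both widgets but shows no step that clears it.
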(event `self.ReceiveBeginPlay`
  (bind _outactors (`GameplayStatics.GetAllActorsOfClass` "/Game/Blueprints/BP_Scoreboard.BP_Scoreboard_C"))
  (for (_array_element _array_index) _outactors
    (switch `int` _array_index
      (:`0`
        (bind _asscoreboard (cast `/Game/GUI/Scoreboard` (`WidgetComponent.GetUserWidgetObject` (`/Game/Blueprints/BP_Scoreboard.Widget` _array_element)) :!pure true))
        (set `self.Scoreboard1Ref` _asscoreboard))
      (:`1`
        (set `self.Scoreboard2Ref` _asscoreboard)))))

(event `AddToScore`
  (params (Score :type Integer))
  (bind _scoreboard1ref (`self.Scoreboard1Ref`))
  (bind _scoreboard2ref (`self.Scoreboard2Ref`))
  ;[1 1 1] Add to score
  (set `self.Score` (+ Score (`self.Score`)))
  (`/Engine/EditorBlueprintResources/StandardMacros.IsValid` _scoreboard1ref
    (:`Is Valid`
      (set `/Game/GUI/Scoreboard.Score` (`self.Score`) _scoreboard1ref))
    (:`Is Not Valid`
      _))
  (`/Engine/EditorBlueprintResources/StandardMacros.IsValid` _scoreboard2ref
    (:`Is Valid`
      (set `/Game/GUI/Scoreboard.Score` (`self.Score`) _scoreboard2ref))))

(event `ResetScore`
  (bind _scoreboard1ref (`self.Scoreboard1Ref`))
  (bind _scoreboard2ref (`self.Scoreboard2Ref`))
  ;[1 1 1] Reset
  (`/Engine/EditorBlueprintResources/StandardMacros.IsValid` _scoreboard1ref
    (:`Is Valid`
      (set `/Game/GUI/Scoreboard.Score` (`self.Score`) _scoreboard1ref))
    (:`Is Not Valid`
      _))
  (`/Engine/EditorBlueprintResources/StandardMacros.IsValid` _scoreboard2ref
    (:`Is Valid`
      (set `/Game/GUI/Scoreboard.Score` (`self.Score`) _scoreboard2ref))))

(fn `UserConstructionScript`)