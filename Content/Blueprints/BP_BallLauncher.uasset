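; BP_BallLauncher is an actor that periodically fires a ball of a configurable type along its forward vector.
; A looping timer starts a timeline that animates the Arrow's X scale, then spawns the ball with a set launch velocity and plays a second scale timeline.
; The construction script pre-fills the Balls array from NumBallsToKeepAlive, and each spawn is written into it, with no explicit destruction of older balls.
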(event `self.ReceiveBeginPlay`
  (`KismetSystemLibrary.K2_SetTimerDelegate` (delegate `LaunchBall`) 5.0 true))

(event `LaunchBall`
  (bind (_direction _newtrack_0) (`Timeline|Timeline_1` :!via `PlayFromStart`)
    (:`Update`
      (`SceneComponent.SetRelativeScale3D` (`self.Arrow`) (`KismetMathLibrary.MakeVector` _newtrack_0 3.0 3.0)))
    (:`Finished`
      (bind _returnvalue (`|SpawnActorFromClass` (`self.BallType`) (`KismetMathLibrary.MakeTransform` (`self.K2_GetActorLocation`)) "AdjustIfPossibleButDontSpawnIfColliding" "OverrideRootScale" null (* (`self.GetActorForwardVector`) (`self.LaunchVelocity`)) null))
      (`KismetArrayLibrary.Array_Set` (`self.Balls`) 0 _returnvalue)
      (bind (_direction_2 _newtrack_0_2) (`Timeline|Timeline_0` :!via `PlayFromStart`)
        (:`Update`
          (`SceneComponent.SetRelativeScale3D` (`self.Arrow`) (`KismetMathLibrary.MakeVector` _newtrack_0_2 3.0 3.0)))))))

(fn `UserConstructionScript`
  (for _ (range 1 (+ (`self.NumBallsToKeepAlive`) 1))
    (`KismetArrayLibrary.Array_Add` (`self.Balls`))))