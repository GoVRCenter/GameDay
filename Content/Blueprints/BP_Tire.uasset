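; BP_Tire is a tire scoring target that celebrates when any actor overlaps its Box trigger.
; An overlap shows the score text and point light, plays jingle and crowd-cheer sounds, and fires every TS_FireworksLauncher in its Fireworks array.
; A timeline raises and scales the text, then hides it with the light and destroys the overlapping actor.
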(event `self.Box.OnComponentBeginOverlap`
  (params (OverlappedComponent :type "PrimitiveComponent Object Reference") (OtherActor :type "Actor Object Reference") (OtherComp :type "PrimitiveComponent Object Reference") (OtherBodyIndex :type Integer) (bFromSweep :type Boolean) (SweepResult :type "HitResult Structure (by ref)"))
  (bind _scoretext (`self.ScoreText`))
  ;[1 1 1] Scoring
  (`SceneComponent.SetVisibility` (`self.PointLight`) true false)
  (`SceneComponent.SetVisibility` (`self.ScoreText`) true false)
  (`GameplayStatics.SpawnSoundAtLocation` "/Game/SFX/WAV/SFX_SuccessJingle.SFX_SuccessJingle" (`self.K2_GetActorLocation`) (struct) 1.0 1.0 0.0 "/Game/SFX/SoundAttenuation.SoundAttenuation" null)
  (`GameplayStatics.PlaySound2D` "/Game/SFX/WAV/SFX_StadiumCrowd_Cheer2.SFX_StadiumCrowd_Cheer2" 1.0 1.0 0.0 null null)
  (`self.FireworksShow`)
  (bind (_direction _animcurve _newtrack_1) (`Timeline|Timeline_0` :!via `PlayFromStart`)
    (:`Update`
      (`SceneComponent.K2_SetRelativeLocation` _scoretext (`KismetMathLibrary.MakeVector` 0.0 95.0 (* _newtrack_1 36.0)) false false)
      (`SceneComponent.SetRelativeScale3D` _scoretext (`KismetMathLibrary.MakeVector` _animcurve _animcurve _animcurve)))
    (:`Finished`
      (`SceneComponent.SetVisibility` (`self.ScoreText`) false false)
      (`SceneComponent.SetVisibility` (`self.PointLight`) false false)
      (`self.K2_DestroyActor` OtherActor))))

(event `FireworksShow`
  ;[1 1 1] Fireworks
  (for _array_element (`self.Fireworks`)
    (bind _asts_fireworks_launcher (cast `/Game/Blueprints/TS_FireworksLauncher` _array_element))
    (`/Game/Blueprints/TS_FireworksLauncher.LaunchShell` _asts_fireworks_launcher)))

(fn `UserConstructionScript`)