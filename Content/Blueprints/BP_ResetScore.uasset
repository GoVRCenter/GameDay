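; BP_ResetScore is a trigger box that resets the game-day score when a master pickup enters it.
; An overlapping pickup is killed and the GameMode_GameDay score is reset, then a jingle and crowd-boo sound play and every launcher in the Fireworks array fires a shell.
; BeginPlay can run the same effects when PreloadPreplayEffects is set.
; An unconnected point-value text update remains in the graph.
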(event `FireworksShow`
  ;[1 1 1] Shoot Fireworks
  (for _array_element (`self.Fireworks`)
    (bind _asts_fireworks_launcher (cast `/Game/Blueprints/TS_FireworksLauncher` _array_element))
    (`/Game/Blueprints/TS_FireworksLauncher.LaunchShell` _asts_fireworks_launcher)))

(event `self.ReceiveBeginPlay`
  ;[0 1 0] Begin Play
  ;[1 1 1] Check for goal
  (if (`self.PreloadPreplayEffects`)
    (`GameplayStatics.PlaySound2D` "/Game/SFX/WAV/SFX_SuccessJingle.SFX_SuccessJingle" 1.0 1.0 0.0 null null :!label _label)
    (`GameplayStatics.SpawnSound2D` "/Game/SFX/WAV/SFX_StadiumCrowd_Boo1.SFX_StadiumCrowd_Boo1" 1.0 1.0 0.0 null)
    (`self.FireworksShow`)))

(event `self.Box1.OnComponentBeginOverlap`
  (params (OverlappedComponent :type "PrimitiveComponent Object Reference") (OtherActor :type "Actor Object Reference") (OtherComp :type "PrimitiveComponent Object Reference") (OtherBodyIndex :type Integer) (bFromSweep :type Boolean) (SweepResult :type "HitResult Structure (by ref)"))
  ;[1 1 1] Check for goal
  (bind _asbp_master_pickup (cast `/Game/Blueprints/Master/BP_MasterPickup` OtherActor))
  (`/Game/Blueprints/Master/BP_MasterPickup.KillItem` _asbp_master_pickup)
  (bind _asgame_mode_game_day (cast `/Game/Blueprints/GameMode_GameDay` (`GameplayStatics.GetGameMode`)))
  (`/Game/Blueprints/GameMode_GameDay.ResetScore` _asgame_mode_game_day)
  (goto _label))

(fn `UserConstructionScript`)