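; Base VR pickup actor that BP_MotionController attaches to a hand socket, then releases with a given velocity and physics re-enabled.
; A looping timer destroys it after a fall out of the world, and KillItem detaches and destroys it after a short delay.
; Hits play a rate-limited bounce sound scaled by impulse strength.
; IsHeld's RepNotify calls SpecialHeldConditions, an empty hook.
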(event `/Game/Blueprints/Data/PickupActorInterface.Pickup`
  (params (AttachTo :type "SceneComponent Object Reference"))
  ;[1 1 1] Pickup drop
  (set `self.IsHeld` true)
  (`PrimitiveComponent.SetSimulatePhysics` (`self.StaticMeshComponent`) false)
  (`SceneComponent.K2_AttachToComponent` (`self.K2_GetRootComponent`) AttachTo "HandSocket" "SnapToTarget" "SnapToTarget" "KeepWorld" true))

(event `self.ReceiveBeginPlay`
  (`KismetSystemLibrary.K2_SetTimerDelegate` (delegate `CheckFall`) 3.0 true)
  (`PrimitiveComponent.SetPhysicsLinearVelocity` (`self.StaticMeshComponent`) (`self.InitialVelocity`) false "None"))

(event `CheckFall`
  (bind (_returnvalue_x _returnvalue_y _returnvalue_z) (`KismetMathLibrary.BreakVector` (`self.K2_GetActorLocation`)))
  (if (< _returnvalue_z -5000.0)
    (`self.K2_DestroyActor`)))

(event `/Game/Blueprints/Data/PickupActorInterface.Drop`
  (params (Velocity :type "Vector Structure"))
  ;[1 1 1] Pickup drop
  (set `self.IsHeld` false)
  (`PrimitiveComponent.SetSimulatePhysics` (`self.StaticMeshComponent`) true)
  (`self.K2_DetachFromActor` "KeepWorld" "KeepWorld" "KeepWorld")
  (`PrimitiveComponent.SetPhysicsLinearVelocity` (`self.StaticMeshComponent`) Velocity false "None")
  (set `self.ThrowLocation` (`self.K2_GetActorLocation`)))

(event `self.ReceiveHit`
  (params (MyComp :type "PrimitiveComponent Object Reference") (Other :type "Actor Object Reference") (OtherComp :type "PrimitiveComponent Object Reference") (bSelfMoved :type Boolean) (HitLocation :type "Vector Structure") (HitNormal :type "Vector Structure") (NormalImpulse :type "Vector Structure") (Hit :type "HitResult Structure (by ref)"))
  (bind _returnvalue (`KismetMathLibrary.VSize` NormalImpulse))
  (bind _audio (`self.Audio`))
  ;[1 1 1] Sound FX for Bounce
  (`/Engine/EditorBlueprintResources/StandardMacros.DoOnce` false :!label _label
    (:`Completed`
      (if (> _returnvalue 60.0)
        (`AudioComponent.SetVolumeMultiplier` _audio (`KismetMathLibrary.MapRangeClamped` _returnvalue 60.0 6000.0 0.1 1.0))
        (`AudioComponent.Play` _audio 0.0))
      (`KismetSystemLibrary.Delay` 0.2)
      (goto _label :!via `Reset`))))

(event `KillItem`
  ;[1 1 1] Destroy
  (`KismetSystemLibrary.Delay` 0.4)
  (`PrimitiveComponent.SetSimulatePhysics` (`self.StaticMeshComponent`) true)
  (`self.K2_DetachFromActor` "KeepWorld" "KeepWorld" "KeepWorld")
  (`self.K2_DestroyActor`))

(event `SpecialHeldConditions`
  (params (IsHeld :type Boolean)))

(fn `OnRep_IsHeld`
  (`self.SpecialHeldConditions` (`self.IsHeld`)))

(fn `UserConstructionScript`
  (`StaticMeshComponent.SetStaticMesh` (`self.StaticMeshComponent`) (`self.BallMesh`)))