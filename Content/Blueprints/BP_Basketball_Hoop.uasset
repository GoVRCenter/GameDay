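; Basketball hoop actor that detects a scored ball and plays the celebration.
; Box1 records the entering master ball and Box2 confirms a goal when that same ball overlaps it, then plays jingle and cheer and destroys the ball after a delay.
; Swoosh plays audio and a DoOnce-gated timeline animating the net material, plus light and points text on a score.
; A separate FireworksShow event launches shells from the Fireworks launchers.
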(event `Swoosh`
  (params (JustScored :type Boolean))
  (bind _pointlight (`self.PointLight`))
  (bind _pointstext (`self.PointsText`))
  ;[1 1 1] Swoosh effects
  (`|ExecutionSequence`
    (:`then_0`
      (`/Engine/EditorBlueprintResources/StandardMacros.DoOnce` false :!label _label
        (:`Completed`
          (if JustScored
            (`SceneComponent.SetVisibility` _pointlight true false)
            (`SceneComponent.SetVisibility` (`self.PointsText`) true false)
            (bind (_direction _animcurve _newtrack_1) (`Timeline|SwooshTimelineAnimation` :!via `PlayFromStart` :!label _label_2)
              (:`Update`
                (`MeshComponent.SetScalarParameterValueOnMaterials` (`self.Net`) "Strength" _animcurve)
                (`SceneComponent.K2_SetRelativeLocation` _pointstext (`KismetMathLibrary.MakeVector` 0.0 95.0 (* _newtrack_1 36.0)) false false)
                (`SceneComponent.SetRelativeScale3D` _pointstext (`KismetMathLibrary.MakeVector` _animcurve _animcurve _animcurve)))
              (:`Finished`
                (`SceneComponent.SetVisibility` _pointlight false false)
                (`SceneComponent.SetVisibility` (`self.PointsText`) false false)
                (goto _label :!via `Reset`)))
            (else
              (goto _label_2 :!via `PlayFromStart`))))))
    (:`then_1`
      (`AudioComponent.Play` (`self.Audio`) 0.0))))

(event `FireworksShow`
  ;[1 1 1] Shoot Fireworks
  (for _array_element (`self.Fireworks`)
    (bind _asts_fireworks_launcher (cast `/Game/Blueprints/TS_FireworksLauncher` _array_element))
    (`/Game/Blueprints/TS_FireworksLauncher.LaunchShell` _asts_fireworks_launcher)))

(event `self.Box1.OnComponentBeginOverlap`
  (params (OverlappedComponent :type "PrimitiveComponent Object Reference") (OtherActor :type "Actor Object Reference") (OtherComp :type "PrimitiveComponent Object Reference") (OtherBodyIndex :type Integer) (bFromSweep :type Boolean) (SweepResult :type "HitResult Structure (by ref)"))
  ;[1 1 1] Check for goal
  (bind _asbp_master_ball (cast `/Game/Blueprints/BP_MasterBall` OtherActor))
  (`/Engine/EditorBlueprintResources/StandardMacros.IsValid` (`self.Box1Ball`)
    (:`Is Not Valid`
      (set `self.Box1Ball` _asbp_master_ball))))

(event `self.Box1.OnComponentEndOverlap`
  (params (OverlappedComponent :type "PrimitiveComponent Object Reference") (OtherActor :type "Actor Object Reference") (OtherComp :type "PrimitiveComponent Object Reference") (OtherBodyIndex :type Integer))
  ;[1 1 1] Check for goal
  (if (== (`self.Box1Ball`) OtherActor)
    (set `self.Box1Ball` null)))

(event `self.Box2.OnComponentBeginOverlap`
  (params (OverlappedComponent :type "PrimitiveComponent Object Reference") (OtherActor :type "Actor Object Reference") (OtherComp :type "PrimitiveComponent Object Reference") (OtherBodyIndex :type Integer) (bFromSweep :type Boolean) (SweepResult :type "HitResult Structure (by ref)"))
  ;[1 1 1] Check for goal
  (cast `/Game/Blueprints/BP_MasterBall` OtherActor)
  (if (== OtherActor (`self.Box1Ball`))
    (`self.Swoosh` true)
    (`GameplayStatics.PlaySound2D` "/Game/SFX/WAV/SFX_SuccessJingle.SFX_SuccessJingle" 1.0 1.0 0.0 null null)
    (if (`KismetMathLibrary.RandomBool`)
      (`GameplayStatics.SpawnSound2D` "/Game/SFX/WAV/SFX_StadiumCrowd_Cheer1.SFX_StadiumCrowd_Cheer1" 1.0 1.0 0.0 null)
      (else
        (`GameplayStatics.SpawnSound2D` "/Game/SFX/WAV/SFX_StadiumCrowd_Cheer1.SFX_StadiumCrowd_Cheer1" 1.0 1.0 0.0 null)))
    (`KismetSystemLibrary.Delay` 1.0)
    (`self.K2_DestroyActor` OtherActor)
    (else
      (`self.Swoosh` false))))

(fn `UserConstructionScript`)